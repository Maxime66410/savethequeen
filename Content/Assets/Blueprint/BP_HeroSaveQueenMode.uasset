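; BP_HeroSaveQueenMode is a Blueprint that persists three Rose values through an SV_SaveData save game.
; On BeginPlay it loads the named slot if it exists, otherwise it creates a fresh SV_SaveData object and saves the current values to that slot.
; LoadData copies the saved Roses into its variables, and SaveCurrentData writes them back to the slot.
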(event `self.ReceiveBeginPlay`
  (bind _returnvalue (`GameplayStatics.DoesSaveGameExist` (`self.SaveName`)))
  (if _returnvalue
    (`self.LoadData`)
    (else
      (bind _returnvalue_2 (`GameplayStatics.CreateSaveGameObject` "/Game/Assets/Blueprint/SV_SaveData.SV_SaveData_C"))
      (bind _assv_save_data (cast `/Game/Assets/Blueprint/SV_SaveData` _returnvalue_2))
      (set `self.SaveData` _assv_save_data)
      (`self.SaveCurrentData`))))

(fn `LoadData`
  (bind _savedata (`self.SaveData`))
  (bind _returnvalue (`GameplayStatics.LoadGameFromSlot` (`self.SaveName`)))
  (bind _assv_save_data (cast `/Game/Assets/Blueprint/SV_SaveData` _returnvalue))
  (set `self.SaveData` _assv_save_data)
  (set `self.Rose1` (`/Game/Assets/Blueprint/SV_SaveData.Rose1` _savedata))
  (set `self.Rose2` (`/Game/Assets/Blueprint/SV_SaveData.Rose2` _savedata))
  (set `self.Rose3` (`/Game/Assets/Blueprint/SV_SaveData.Rose3` _savedata)))

(fn `SaveCurrentData`
  (bind _savedata (`self.SaveData`))
  (set `/Game/Assets/Blueprint/SV_SaveData.Rose1` (`self.Rose1`) _savedata)
  (set `/Game/Assets/Blueprint/SV_SaveData.Rose2` (`self.Rose2`) _savedata)
  (set `/Game/Assets/Blueprint/SV_SaveData.Rose3` (`self.Rose3`) _savedata)
  (`GameplayStatics.SaveGameToSlot` (`self.SaveData`) (`self.SaveName`)))

(fn `UserConstructionScript`)