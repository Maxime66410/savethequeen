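; BP_Ambient is a music actor that plays an ambient sound for the level.
; On BeginPlay it assigns its Sound to the Audio component and starts playback.
; A self-calling SyncMusic event checks every 0.2 seconds and restarts the audio from the beginning whenever it has stopped, so the sound loops continuously.
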(event `self.ReceiveBeginPlay`
  (`AudioComponent.SetSound` (`self.Audio`) (`self.Sound`))
  (`AudioComponent.Play` (`self.Audio`) 0.0)
  (`self.SyncMusic`))

(event `SyncMusic`
  (if (not (`AudioComponent.IsPlaying` (`self.Audio`)))
    (`AudioComponent.Play` (`self.Audio`) 0.0))
  (`KismetSystemLibrary.Delay` 0.2)
  (`self.SyncMusic`))

(fn `UserConstructionScript`)