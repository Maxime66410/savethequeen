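; BP_EndLvl1 is the level 1 end trigger, which also deals 1000 damage to overlapping enemies.
; When the hero knight enters, it disables input and reveals the Rose with a timeline-driven scale animation.
; It then sets a Rose flag in a loaded or newly created SV_SaveData and opens MAP_Menu.
; The save object is not written back to its slot here.
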(event `self.Trigger.OnComponentBeginOverlap`
  (params (OverlappedComponent :type "PrimitiveComponent Object Reference") (OtherActor :type "Actor Object Reference") (OtherComp :type "PrimitiveComponent Object Reference") (OtherBodyIndex :type Integer) (bFromSweep :type Boolean) (SweepResult :type "HitResult Structure (by ref)"))
  (bind _asplayer_hero_knight (cast `/Game/Assets/Blueprint/Player/PlayerHeroKnight` OtherActor)
    (:`then`
      (`self.DisableInput` _asplayer_hero_knight (`GameplayStatics.GetPlayerController` 0))
      (`self.Animation_Size`))
    (:`CastFailed`
      (bind _asbp_ennemie (cast `/Game/Assets/Blueprint/IA/BP_Ennemie` OtherActor))
      (`/Game/Assets/Blueprint/IA/BP_Ennemie.GetDamaged` _asbp_ennemie 1000.0))))

(event `Animation_Size`
  (bind _rose (`self.Rose`))
  (`SceneComponent.SetVisibility` _rose true false)
  (bind (_direction _changesize) (`Timeline|SizeChange`)
    (:`Update`
      (`SceneComponent.SetWorldScale3D` _rose (`KismetMathLibrary.MakeVector` _changesize _changesize _changesize)))
    (:`Finished`
      (`self.SaveData`))))

(event `SaveData`
  (bind _returnvalue (`GameplayStatics.DoesSaveGameExist` (`self.Slot Name`)))
  (if _returnvalue
    (bind _returnvalue_2 (`GameplayStatics.LoadGameFromSlot` (`self.Slot Name`)))
    (bind _assv_save_data (cast `/Game/Assets/Blueprint/SV_SaveData` _returnvalue_2))
    (set `self.Save` _assv_save_data)
    (else
      (bind _returnvalue_3 (`GameplayStatics.CreateSaveGameObject` "/Game/Assets/Blueprint/SV_SaveData.SV_SaveData_C"))
      (set `self.Save` _returnvalue_3)))
  (`KismetArrayLibrary.Array_Set` (`/Game/Assets/Blueprint/SV_SaveData.Rose` (`self.Save`)) 0 true)
  (`self.LoadMenu`))

(event `LoadMenu`
  (`GameplayStatics.OpenLevel` "MAP_Menu"))

(fn `UserConstructionScript`)