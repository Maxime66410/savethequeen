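; BP_Respawn is a one-time checkpoint that moves the respawn point when a living PlayerHeroKnight enters its trigger.
; The overlap sets the trigger to ignore all channels, replaces the PlayerStart, plays a bonfire sound and heals the knight.
; Replacement destroys the first PlayerStart found in the level, then spawns a new one at the PointStart component's location, unless it would collide.
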(event `self.Trigger.OnComponentBeginOverlap`
  (params (OverlappedComponent :type "PrimitiveComponent Object Reference") (OtherActor :type "Actor Object Reference") (OtherComp :type "PrimitiveComponent Object Reference") (OtherBodyIndex :type Integer) (bFromSweep :type Boolean) (SweepResult :type "HitResult Structure (by ref)"))
  ;[1 1 1] On Collision
  (bind _asplayer_hero_knight (cast `/Game/Assets/Blueprint/Player/PlayerHeroKnight` OtherActor))
  (set `self.As Player Hero Knight` _asplayer_hero_knight)
  (if (not (`/Game/Assets/Blueprint/Player/PlayerHeroKnight.IsDeath` _asplayer_hero_knight))
    (`self.DisabledCollision`)))

(event `DisabledCollision`
  (bind _as_player_hero_knight (`self.As Player Hero Knight`))
  ;[1 1 1] Change Collision Settings
  (`PrimitiveComponent.SetCollisionResponseToAllChannels` (`self.Trigger`) "ECR_Ignore")
  (`self.LoadNewPlayerStart`)
  (`GameplayStatics.PlaySound2D` "/Game/Assets/Audio/SFX/dark-souls-bonfire-sound-effect.dark-souls-bonfire-sound-effect" 0.4 1.0 0.0 null null)
  (`/Engine/EditorBlueprintResources/StandardMacros.IsValid` _as_player_hero_knight
    (:`Is Valid`
      (`/Game/Assets/Blueprint/Player/PlayerHeroKnight.Heal` _as_player_hero_knight 50.0))))

(event `LoadNewPlayerStart`
  ;[1 1 1] Destroy Old Start
  (bind _outactors (`GameplayStatics.GetAllActorsOfClass` "/Script/Engine.PlayerStart"))
  (for _array_element _outactors
    (`self.K2_DestroyActor` _array_element)
    (break))
  (`self.MakeNewPlayerStart`))

(event `MakeNewPlayerStart`
  ;[1 1 1] Instance new Actor
  (`|SpawnActorFromClass` "/Script/Engine.PlayerStart" (`KismetMathLibrary.Conv_VectorToTransform` (`SceneComponent.K2_GetComponentLocation` (`self.PointStart`))) "DontSpawnIfColliding" "OverrideRootScale" null null))

(fn `UserConstructionScript`)