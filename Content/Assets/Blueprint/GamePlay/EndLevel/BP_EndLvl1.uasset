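; BP_EndLvl1 is the level 1 end trigger that awards the rose and returns the player to the menu.
; Hero overlap disables input, then reveals and scales the Rose through a timeline with sound; overlapping enemies instead take massive damage.
; When the animation finishes, it plays the victory sound, loads or creates the save object, flags Rose1 on the game mode, saves, then opens MAP_Menu after a delay.
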(event `self.Trigger.OnComponentBeginOverlap`
  (params (OverlappedComponent :type "PrimitiveComponent Object Reference") (OtherActor :type "Actor Object Reference") (OtherComp :type "PrimitiveComponent Object Reference") (OtherBodyIndex :type Integer) (bFromSweep :type Boolean) (SweepResult :type "HitResult Structure (by ref)"))
  (bind _asplayer_hero_knight (cast `/Game/Assets/Blueprint/Player/PlayerHeroKnight` OtherActor)
    (:`then`
      (`KismetSystemLibrary.Delay` 0.2)
      (`self.DisableInput` _asplayer_hero_knight (`GameplayStatics.GetPlayerController` 0))
      (`self.Animation_Size`))
    (:`CastFailed`
      (bind _asbp_ennemie (cast `/Game/Assets/Blueprint/IA/BP_Ennemie` OtherActor))
      (`/Game/Assets/Blueprint/IA/BP_Ennemie.GetDamaged` _asbp_ennemie 1000.0))))

(event `Animation_Size`
  (bind _rose (`self.Rose`))
  (`GameplayStatics.SpawnSound2D` "/Game/Assets/Audio/Menu/079_Buy_sell_01.079_Buy_sell_01" 1.0 1.0 0.0 null)
  (`SceneComponent.SetVisibility` _rose true false)
  (bind (_direction _changesize) (`Timeline|SizeChange`)
    (:`Update`
      (`SceneComponent.SetWorldScale3D` _rose (`KismetMathLibrary.MakeVector` _changesize _changesize _changesize)))
    (:`Finished`
      (`self.SaveData`))))

(event `SaveData`
  (`GameplayStatics.SpawnSound2D` "/Game/Assets/Audio/SFX/victory_SoundEffect.victory_SoundEffect" 1.0 1.0 0.0 null)
  (bind _returnvalue (`GameplayStatics.DoesSaveGameExist` (`self.Slot Name`)))
  (if _returnvalue
    (bind _returnvalue_2 (`GameplayStatics.LoadGameFromSlot` (`self.Slot Name`)))
    (bind _assv_save_data (cast `/Game/Assets/Blueprint/SV_SaveData` _returnvalue_2))
    (set `self.Save` _assv_save_data)
    (else
      (bind _returnvalue_3 (`GameplayStatics.CreateSaveGameObject` "/Game/Assets/Blueprint/SV_SaveData.SV_SaveData_C"))
      (set `self.Save` _returnvalue_3)))
  (bind _asbp_hero_save_queen_mode (cast `/Game/Assets/Blueprint/BP_HeroSaveQueenMode` (`GameplayStatics.GetGameMode`)))
  (set `/Game/Assets/Blueprint/BP_HeroSaveQueenMode.Rose1` true _asbp_hero_save_queen_mode)
  (`/Game/Assets/Blueprint/BP_HeroSaveQueenMode.SaveCurrentData` _asbp_hero_save_queen_mode)
  (`self.LoadMenu`))

(event `LoadMenu`
  (`KismetSystemLibrary.Delay` 5.0)
  (`GameplayStatics.OpenLevel` "MAP_Menu"))

(fn `UserConstructionScript`)