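; Trigger volume that starts the boss encounter when the player's hero knight enters it.
; On overlap it disables its box collision, plays a wide camera shake at the knight and adds a force feedback component.
; After a short delay it activates the boss found at BeginPlay, adds its interface, tells the combat audio actor to enable boss mode, then destroys itself.
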(event `self.ReceiveBeginPlay`
  (bind _returnvalue (`GameplayStatics.GetActorOfClass` "/Game/Assets/Blueprint/IA/Boss/BP_Boss.BP_Boss_C"))
  (set `self.Boss` _returnvalue)
  (bind _returnvalue_2 (`GameplayStatics.GetActorOfClass` "/Game/Assets/Blueprint/Environment/Niv3/BP_AudioCombat.BP_AudioCombat_C"))
  (set `self.AudioCombat` _returnvalue_2))

(event `AppealBoss`
  (bind _boss (`self.Boss`))
  (set `/Game/Assets/Blueprint/IA/Boss/BP_Boss.IsActive` true _boss)
  (`/Game/Assets/Blueprint/IA/Boss/BP_Boss.AddInterface` _boss))

(event `self.Box.OnComponentBeginOverlap`
  (params (OverlappedComponent :type "PrimitiveComponent Object Reference") (OtherActor :type "Actor Object Reference") (OtherComp :type "PrimitiveComponent Object Reference") (OtherBodyIndex :type Integer) (bFromSweep :type Boolean) (SweepResult :type "HitResult Structure (by ref)"))
  (bind _asplayer_hero_knight (cast `/Game/Assets/Blueprint/Player/PlayerHeroKnight` OtherActor))
  (set `self.As Player Hero Knight` _asplayer_hero_knight)
  (`PrimitiveComponent.SetCollisionResponseToAllChannels` (`self.Box`) "ECR_Ignore")
  (`self.Tremblement`)
  (`KismetSystemLibrary.Delay` 3.0)
  (`self.AppealBoss`)
  (`self.EnabledBoss`)
  (`self.K2_DestroyActor`))

(event `Tremblement`
  (`GameplayStatics.PlayWorldCameraShake` "/Game/Assets/Blueprint/FeedBack/CS_BossDisplay.CS_BossDisplay_C" (`self.K2_GetActorLocation` (`self.As Player Hero Knight`)) 100000.0)
  (`AddComponent|NODE_AddForceFeedbackComponent-0`))

(event `EnabledBoss`
  (`/Game/Assets/Blueprint/Environment/Niv3/BP_AudioCombat.EnableBoss` (`self.AudioCombat`)))

(fn `UserConstructionScript`)