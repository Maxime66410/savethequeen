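; BP_TeleportSpawner is a one-shot actor that shows a teleport effect and spawns a BP_Ennemie at its own transform.
; On BeginPlay, a timed chain of delays switches the Teleport flipbook from opening to looping to closing animations.
; The enemy appears during the loop phase, and the actor destroys itself once the closing animation has had time to play.
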(event `self.ReceiveBeginPlay`
  (`PaperFlipbookComponent.SetFlipbook` (`self.Teleport`) "/Game/Assets/Sprite/Ennemy/Teleport/FP_TeleportStart.FP_TeleportStart")
  (`KismetSystemLibrary.Delay` 0.4)
  (`PaperFlipbookComponent.SetFlipbook` (`self.Teleport`) "/Game/Assets/Sprite/Ennemy/Teleport/FP_TeleportLoop.FP_TeleportLoop")
  (`KismetSystemLibrary.Delay` 3.0)
  (`|SpawnActorFromClass` "/Game/Assets/Blueprint/IA/BP_Ennemie.BP_Ennemie_C" (`self.GetTransform`) "Undefined" "OverrideRootScale" null null)
  (`KismetSystemLibrary.Delay` 2.0)
  (`PaperFlipbookComponent.SetFlipbook` (`self.Teleport`) "/Game/Assets/Sprite/Ennemy/Teleport/FP_TeleportClose.FP_TeleportClose")
  (`KismetSystemLibrary.Delay` 0.5)
  (`self.K2_DestroyActor`))

(fn `UserConstructionScript`)