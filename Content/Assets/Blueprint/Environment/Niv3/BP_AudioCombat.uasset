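; BP_AudioCombat is a level 3 environment Blueprint that controls ambient and boss fight music through three audio components.
; On BeginPlay, SoundBackground plays a strings ambience layer.
; EnableBoss plays a battle intro on SoundEffect, fades out the ambience with a delayed stop, and after a short delay starts the battle loop on SoundMusic.
; FinishBoss stops that loop and plays the ending stinger on SoundEffect.
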(event `self.ReceiveBeginPlay`
  (bind _soundbackground (`self.SoundBackground`))
  (`AudioComponent.SetSound` _soundbackground "/Game/Assets/Audio/Ambient/Niv3/ambience_04_LAYER_A_strings.ambience_04_LAYER_A_strings")
  (`AudioComponent.Play` _soundbackground 0.0))

(event `EnableBoss`
  (bind _soundeffect (`self.SoundEffect`))
  (`AudioComponent.SetSound` _soundeffect "/Game/Assets/Audio/Ambient/Niv3/bigbattle_1_LOOP_START.bigbattle_1_LOOP_START")
  (`AudioComponent.Play` _soundeffect 0.0)
  (`AudioComponent.StopDelayed` (`self.SoundBackground`) 2.0)
  (`KismetSystemLibrary.Delay` 0.8)
  (`self.SetMusicBoss`))

(event `SetMusicBoss`
  (bind _soundmusic (`self.SoundMusic`))
  (`AudioComponent.SetSound` _soundmusic "/Game/Assets/Audio/Ambient/Niv3/bigbattle_2_LOOP.bigbattle_2_LOOP")
  (`AudioComponent.Play` _soundmusic 0.0))

(event `FinishBoss`
  (bind _soundeffect (`self.SoundEffect`))
  (`AudioComponent.Stop` (`self.SoundMusic`))
  (`AudioComponent.SetSound` _soundeffect "/Game/Assets/Audio/Ambient/Niv3/bigbattle_2_LOOP_END_1.bigbattle_2_LOOP_END_1")
  (`AudioComponent.Play` _soundeffect 0.0))

(fn `UserConstructionScript`)