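; BP_SpawnLeaf is a level 1 environment spawner that periodically launches leaf actors.
; After a short random delay at BeginPlay, the SpawnLeaf event spawns a BP_Leaf at its Arrow component's location, skipping spawns that would collide.
; It pushes the leaf's PaperSprite with a physics impulse along negative world X, then re-calls itself after a random delay, looping indefinitely.
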(event `self.ReceiveBeginPlay`
  (`KismetSystemLibrary.Delay` (`KismetMathLibrary.RandomFloatInRange` 1.0 2.0))
  (`self.SpawnLeaf`))

(event `SpawnLeaf`
  (bind _returnvalue (`|SpawnActorFromClass` "/Game/Assets/Blueprint/Environment/Niv1/BP_Leaf.BP_Leaf_C" (`KismetMathLibrary.Conv_VectorToTransform` (`SceneComponent.K2_GetComponentLocation` (`self.Arrow`))) "DontSpawnIfColliding" "OverrideRootScale" null null))
  (`PrimitiveComponent.AddImpulse` (`/Game/Assets/Blueprint/Environment/Niv1/BP_Leaf.PaperSprite` _returnvalue) (-1000.0 0.0 0.0) "None" false)
  (`KismetSystemLibrary.Delay` (`KismetMathLibrary.RandomFloatInRange` 2.0 8.0))
  (`self.SpawnLeaf`))

(fn `UserConstructionScript`)