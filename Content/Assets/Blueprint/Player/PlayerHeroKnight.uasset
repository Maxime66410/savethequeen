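; Player knight for a 2D side-scroller, a Paper2D character that runs, jumps, attacks, blocks, rolls, takes damage and respawns at a PlayerStart.
; State booleans gate input and the flipbook chosen on Tick, which also turns the controller toward the movement direction.
; Attacks briefly enable an overlap box that damages enemies and bosses; rolls launch the knight with damage and Pawn collision off.
; A self-repeating delayed event plays footsteps.
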(event `InputAction|Attack`
  (params (Key :type "Key Structure"))
  (bind _attackstates (`self.AttackStates`))
  ;[1 0.6558 0.4623] Attack
  (:`Pressed`
    (if (not (`self.IsDeath`))
      (if (not (`self.IsAttack`))
        (`GameplayStatics.PlaySound2D` "/Game/Assets/Audio/SFX/Battle/03_Claw_03.03_Claw_03" 0.5 (`KismetMathLibrary.RandomFloatInRange` 0.8 1.2) 0.0 null null)
        (set `self.IsAttack` true)
        (`PrimitiveComponent.SetCollisionResponseToChannel` (`self.TriggerAttackBox`) "ECC_Pawn" "ECR_Overlap")
        (`PaperFlipbookComponent.SetFlipbook` (`self.Sprite`) (`|GetArrayItem` _attackstates (`KismetMathLibrary.RandomIntegerInRange` 0 (- (`KismetArrayLibrary.Array_Length` _attackstates) 1))))
        (`KismetSystemLibrary.Delay` 0.3)
        (set `self.IsAttack` false)
        (`PrimitiveComponent.SetCollisionResponseToAllChannels` (`self.TriggerAttackBox`) "ECR_Ignore")))))

(event `InputAction|Block`
  (params (Key :type "Key Structure"))
  (bind _returnvalue (not (`self.IsDeath`)))
  ;[0.8025 0.6249 1] Block Attack
  (:`Pressed`
    (if _returnvalue
      (set `self.IsBlock` true)
      (`PaperFlipbookComponent.SetFlipbook` (`self.Sprite`) "/Game/Assets/Sprite/Player/BlockIdle/HeroKnight_Block_Idle.HeroKnight_Block_Idle")))
  (:`Released`
    (if _returnvalue
      (set `self.IsBlock` false))))

(event `UpdateAnimation`
  ;[0.5728 0.9901 1] Handle Animation
  (if (not (`self.IsDeath`))
    (if (not (`self.IsRoll`))
      (if (not (`self.IsAttack`))
        (if (not (`self.IsBlock`))
          (if (not (`self.IsGetDamaged`))
            (`PaperFlipbookComponent.SetFlipbook` (`self.Sprite`) (select `bool` (`NavMovementComponent.IsFalling` (`self.CharacterMovement`)) :`false` (select `bool` (> (`KismetMathLibrary.VSize` (`self.GetVelocity`)) 0.0) :`false` "/Game/Assets/Sprite/Player/Idle/HeroKnight_Idle.HeroKnight_Idle" :`true` "/Game/Assets/Sprite/Player/Run/HeroKnight_Run.HeroKnight_Run" :!type "PaperFlipbook Object Reference") :`true` "/Game/Assets/Sprite/Player/Fall/HeroKnight_Fall.HeroKnight_Fall"))))))))

(event `InputAction|Roll`
  (params (Key :type "Key Structure"))
  (bind _returnvalue_x (`KismetMathLibrary.BreakVector` (`KismetMathLibrary.GetForwardVector` (`SceneComponent.K2_GetComponentRotation` (`self.CapsuleComponent`)))))
  ;[0.9879 1 0.4779] Roll
  (:`Pressed`
    (if (not (`self.IsDeath`))
      (if (not (`NavMovementComponent.IsFalling` (`self.CharacterMovement`)))
        (if (not (`self.IsRoll`))
          (`GameplayStatics.PlaySound2D` "/Game/Assets/Audio/SFX/Battle/51_Flee_02.51_Flee_02" 0.8 1.0 0.0 null null)
          (`PrimitiveComponent.SetCollisionResponseToChannel` (`self.CapsuleComponent`) "ECC_Pawn" "ECR_Ignore")
          (set `self.CanGetDamage` false)
          (set `self.IsRoll` true)
          (`self.LaunchCharacter` (`KismetMathLibrary.MakeVector` (* _returnvalue_x 2000.0)))
          (`PaperFlipbookComponent.SetFlipbook` (`self.Sprite`) "/Game/Assets/Sprite/Player/Roll/HeroKnight_Roll.HeroKnight_Roll")
          (`KismetSystemLibrary.Delay` 0.5)
          (set `self.IsRoll` false)
          (set `self.CanGetDamage` true)
          (`PrimitiveComponent.SetCollisionResponseToChannel` (`self.CapsuleComponent`) "ECC_Pawn" "ECR_Block"))))))

(event `StepPlayer`
  ;[1 0.3604 0.5318] Step System
  (if (and (`self.IsMove`) (not (`NavMovementComponent.IsFalling` (`self.CharacterMovement`))) (not (`self.IsDeath`)))
    (`GameplayStatics.PlaySound2D` "/Game/Assets/Audio/SFX/Movement/03_Step_grass_03.03_Step_grass_03" 0.3 (`KismetMathLibrary.RandomFloatInRange` 0.5 1.5) 0.0 null null))
  (`KismetSystemLibrary.Delay` 0.3)
  (`self.StepPlayer`))

(event `self.ReceiveTick`
  (params (DeltaSeconds :type "Float (single-precision)"))
  (bind _returnvalue (`self.GetController`))
  (bind _returnvalue_2 (`self.GetController`))
  ;[0.625 1 0.555] Tick - Updates animation
  (`self.UpdateAnimation`)
  (if (not (`self.IsRoll`))
    (if (not (`self.IsBlock`))
      (`/Engine/EditorBlueprintResources/StandardMacros.CompareFloat` (.x (`MovementComponent.Velocity` (`self.GetMovementComponent`)))
        (:`>`
          (`/Engine/EditorBlueprintResources/StandardMacros.IsValid` _returnvalue_2 :!label _label
            (:`Is Valid`
              (`Controller.SetControlRotation` _returnvalue_2 (`KismetMathLibrary.MakeRotator` 0.0)))))
        (:`==`
          (if (`self.bisMovingRight`)
            (goto _label)
            (else
              (`/Engine/EditorBlueprintResources/StandardMacros.IsValid` _returnvalue :!label _label_2
                (:`Is Valid`
                  (`Controller.SetControlRotation` _returnvalue (`KismetMathLibrary.MakeRotator` 0.0 0.0 180.0)))))))
        (:`<`
          (goto _label_2)))
      (else
        ;;[0 0 0] Debug block animation
        (`KismetSystemLibrary.Delay` 0.5)
        (set `self.IsBlock` false)))
    (else
      (`KismetSystemLibrary.Delay` 0.5)
      (set `self.IsRoll` false))))

(event `InputAxis|MoveRight`
  (params (AxisValue :type "Float (single-precision)"))
  ;[0.865 0.7699 1] Handle movement
  (if (not (`self.IsDeath`))
    (if (not (`self.IsRoll`))
      (if (not (`self.IsBlock`))
        (if (> AxisValue 0.0)
          (set `self.bisMovingRight` true)
          (elif (< AxisValue 0.0)
            (set `self.bisMovingRight` false)))
        (`self.AddMovementInput` (1.0 0.0 0.0) AxisValue)
        (if (!= AxisValue 0.0)
          (set `self.IsMove` true)
          (else
            (set `self.IsMove` false)))))))

(event `InputAction|Jump`
  (params (Key :type "Key Structure"))
  ;[0.4828 1 0.7041] Handle Jump
  (:`Pressed`
    (if (not (`self.IsDeath`)) :!label _label_3
      (if (not (`self.IsBlock`))
        (if (not (`self.IsJump`))
          (`self.Jump`)
          (`GameplayStatics.PlaySound2D` "/Game/Assets/Audio/SFX/Movement/30_Jump_03.30_Jump_03" 0.5 1.0 0.0 null null)
          (set `self.IsJump` true)
          (`PaperFlipbookComponent.SetFlipbook` (`self.Sprite`) "/Game/Assets/Sprite/Player/Jump/HeroKnight_Jump.HeroKnight_Jump")))))
  (:`Released`
    (`self.StopJumping` :!label _label_4)))

(event `InputTouch`
  (params (Location :type "Vector Structure") (FingerIndex :type "ETouchIndex Enum"))
  ;[0.4828 1 0.7041] Handle Jump
  (:`Pressed`
    (goto _label_3))
  (:`Released`
    (goto _label_4)))

(event `self.CapsuleComponent.OnComponentHit`
  (params (HitComponent :type "PrimitiveComponent Object Reference") (OtherActor :type "Actor Object Reference") (OtherComp :type "PrimitiveComponent Object Reference") (NormalImpulse :type "Vector Structure") (Hit :type "HitResult Structure (by ref)"))
  ;[0.4828 1 0.7041] Handle Jump
  ;;[0.1896 1 0.2863] Reset Jump
  (cast `/Game/Assets/Blueprint/IA/BP_Ennemie` OtherActor
    (:`CastFailed`
      (if (`self.IsJump`)
        (set `self.IsJump` false)
        (`GameplayStatics.PlaySound2D` "/Game/Assets/Audio/SFX/Movement/45_Landing_01.45_Landing_01" 0.5 1.0 0.0 null null)))))

(event `GetDamaged`
  (params (Damage :type "Float (double-precision)"))
  ;[1 0.2603 0] Get Damage
  (if (not (`self.IsDeath`))
    (if (`self.CanGetDamage`)
      (if (not (`self.IsBlock`))
        (`GameplayStatics.PlaySound2D` "/Game/Assets/Audio/SFX/Movement/61_Hit_03.61_Hit_03" 1.0 (`KismetMathLibrary.RandomFloatInRange` 0.8 1.2) 0.0 null null)
        (set `self.IsGetDamaged` true)
        (`PaperFlipbookComponent.SetFlipbook` (`self.Sprite`) "/Game/Assets/Sprite/Player/Hurt/HeroKnight_Hurt.HeroKnight_Hurt")
        (set `self.Health` (- (`self.Health`) Damage))
        (`KismetSystemLibrary.Delay` 0.2)
        (set `self.IsGetDamaged` false)
        ;[1 0.1407 0.2304] Check if dead
        (if (>= 0.0 (`self.Health`))
          (`GameplayStatics.PlaySound2D` "/Game/Assets/Audio/SFX/Battle/69_Enemy_death_01.69_Enemy_death_01" 1.0 1.0 0.0 null null)
          (set `self.IsDeath` true)
          (`PaperFlipbookComponent.SetFlipbook` (`self.Sprite`) "/Game/Assets/Sprite/Player/Death/HeroKnight_Death.HeroKnight_Death")
          (`KismetSystemLibrary.Delay` 0.9)
          (`PaperFlipbookComponent.SetFlipbook` (`self.Sprite`) "/Game/Assets/Sprite/Player/Death/HeroKnight_Death_Loop.HeroKnight_Death_Loop")
          (`KismetSystemLibrary.Delay` 3.0)
          (`self.Respawn`))
        (else
          (`PaperFlipbookComponent.SetFlipbook` (`self.Sprite`) "/Game/Assets/Sprite/Player/Block/HeroKnight_Block.HeroKnight_Block")
          (`GameplayStatics.PlaySound2D` "/Game/Assets/Audio/SFX/Movement/61_Hit_03.61_Hit_03" 1.0 (`KismetMathLibrary.RandomFloatInRange` 0.2 0.4) 0.0 null null)
          (`KismetSystemLibrary.Delay` 0.2)
          (set `self.IsBlock` false)
          (`KismetSystemLibrary.Delay` 0.2)
          (set `self.IsBlock` true)
          (`PaperFlipbookComponent.SetFlipbook` (`self.Sprite`) "/Game/Assets/Sprite/Player/BlockIdle/HeroKnight_Block_Idle.HeroKnight_Block_Idle"))))))

(event `self.ReceiveBeginPlay`
  (`ActorComponent.SetIsReplicated` (`self.Sprite`) true)
  (`self.StepPlayer`))

(event `Respawn`
  ;[0 0 0] Respawn System
  (bind _outactors (`GameplayStatics.GetAllActorsOfClass` "/Script/Engine.PlayerStart"))
  (for _array_element _outactors
    (set `self.RespawnStart` _array_element)
    (break))
  (`SceneComponent.K2_SetWorldLocation` (`self.CapsuleComponent`) (`self.K2_GetActorLocation` (`self.RespawnStart`)) false true)
  (set `self.Health` 100.0)
  (set `self.IsDeath` false))

(event `Heal`
  (params (AddHeal :type "Float (double-precision)"))
  ;[1 1 1] Heal Player
  (set `self.Health` (+ (`self.Health`) AddHeal)))

(event `self.TriggerAttackBox.OnComponentBeginOverlap`
  (params (OverlappedComponent :type "PrimitiveComponent Object Reference") (OtherActor :type "Actor Object Reference") (OtherComp :type "PrimitiveComponent Object Reference") (OtherBodyIndex :type Integer) (bFromSweep :type Boolean) (SweepResult :type "HitResult Structure (by ref)"))
  ;[1 1 1] Attack Box
  (bind _asbp_ennemie (cast `/Game/Assets/Blueprint/IA/BP_Ennemie` OtherActor)
    (:`then`
      (`/Game/Assets/Blueprint/IA/BP_Ennemie.GetDamaged` _asbp_ennemie (`KismetMathLibrary.RandomFloatInRange` 12.5 20.0)))
    (:`CastFailed`
      (bind _asbp_boss (cast `/Game/Assets/Blueprint/IA/Boss/BP_Boss` OtherActor))
      (`/Game/Assets/Blueprint/IA/Boss/BP_Boss.Get Damaged Boss` _asbp_boss (`KismetMathLibrary.RandomFloatInRange` 12.5 30.0)))))

(event `InputAction|DebugDamage`
  (params (Key :type "Key Structure"))
  (:`Pressed`
    (`self.GetDamaged` 50.0)))

(fn `UserConstructionScript`)