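; Paper2D boss with a head and two hands that trails the player while active and takes damage until death.
; Tick drives a random behaviour pick between idling, spawning a teleport spawner at the player, or a hand punch.
; Punches track the player, flash eyes, then slam down with overlap damage to player and enemies, all via interpolation.
; Death sinks the boss, swaps materials, spawns a flower and kills all enemies.
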(event `NeutralEvent`
  ;[1 0.8425 0] Neutral AI
  (if (not (`self.IsNeutral`))
    (set `self.IsNeutral` true)
    (`KismetSystemLibrary.Delay` (`KismetMathLibrary.RandomFloatInRange` 5.0 15.0))
    (set `self.IsChooseAttack` false)
    (set `self.IsNeutral` false)))

(event `AddInterface`
  ;[1 0.352 0.3222] Add interface
  (bind _returnvalue (`|CreateWidget` "/Game/Assets/Sprite/UI/Boss/User_BossInterface.User_BossInterface_C"))
  (`/Game/Assets/Sprite/UI/Boss/User_BossInterface.SetupBoss` _returnvalue self)
  (`UserWidget.AddToViewport` _returnvalue 0))

(event `SpawnNPC`
  (bind (_returnvalue_x _returnvalue_y _returnvalue_z) (`KismetMathLibrary.BreakVector` (`SceneComponent.K2_GetComponentLocation` (`PaperCharacter.Sprite` (`self.As Player Hero Knight`)))))
  ;[0.2648 0.7458 1] Spawn NPC
  (if (not (`self.IsSpawnNPC`))
    (set `self.IsSpawnNPC` true)
    (`self.DebugResetLR`)
    (`|SpawnActorFromClass` "/Game/Assets/Blueprint/GamePlay/BP_TeleportSpawner.BP_TeleportSpawner_C" (`KismetMathLibrary.MakeTransform` (`KismetMathLibrary.MakeVector` _returnvalue_x _returnvalue_y (* _returnvalue_z 1.0))) "Undefined" "OverrideRootScale" null null)
    (`KismetSystemLibrary.Delay` (`KismetMathLibrary.RandomFloatInRange` 5.0 15.0))
    (set `self.IsChooseAttack` false)
    (set `self.IsSpawnNPC` false)))

(event `WantAttack`
  ;[0.2396 0.06806 0] Choose Random Behaviour
  (if (not (`self.IsChooseAttack`))
    (set `self.IsChooseAttack` true)
    (bind _output_get (set `self.RandomIntAttack` (select `bool` (`self.IsFirstTime?`) :`false` (`KismetMathLibrary.RandomIntegerInRange` 0 5))))
    (set `self.IsFirstTime?` false)
    (switch `int` _output_get
      (:`Default`
        (set `self.BehaviourAI` "NewEnumerator0" :!label _label))
      (:`0`
        (goto _label))
      (:`1`
        (set `self.BehaviourAI` "NewEnumerator1" :!label _label_2))
      (:`2`
        (goto _label))
      (:`3`
        (set `self.BehaviourAI` "NewEnumerator2" :!label _label_3))
      (:`4`
        (goto _label_2))
      (:`5`
        (goto _label_3)))
    (switch `/Game/Assets/Blueprint/IA/Boss/BossAttackType` (`self.BehaviourAI`)
      (:`NewEnumerator0`
        (`self.NeutralEvent`))
      (:`NewEnumerator1`
        (`self.HandPreparationAndAttack`))
      (:`NewEnumerator2`
        (`self.SpawnNPC`)))
    (elif (`self.IsPreprepared`)
      (`self.HandPreparationAndAttack`))))

(event `self.ReceiveBeginPlay`
  (bind _asplayer_hero_knight (cast `/Game/Assets/Blueprint/Player/PlayerHeroKnight` (`GameplayStatics.GetPlayerPawn` 0)))
  (set `self.As Player Hero Knight` _asplayer_hero_knight)
  (`self.DisableCollision`)
  (`PaperFlipbookComponent.SetLooping` (`self.Eyeflink`) false))

(event `DebugResetLR`
  ;[0.4531 0.4531 0.4531] Debug Reset
  (`self.DisableCollision`)
  (set `self.BehaviourAI` "NewEnumerator0")
  (set `self.BossAttackHand` "NewEnumerator0")
  (set `self.IsRandomSideChoose` false)
  (set `self.IsPreprepared` false))

(event `self.ReceiveTick`
  (params (DeltaSeconds :type "Float (single-precision)"))
  (set `self.Delta Seconds` DeltaSeconds)
  (if (`self.IsActive`)
    (if (not (`self.IsDeath`))
      (`self.FollowPlayer`)
      (`self.HandLTransformFreeze`)
      (`self.HandRTransformFreeze`)
      (`self.WantAttack`)
      (else
        (`self.DeathGoDown`)
        (`/Engine/EditorBlueprintResources/StandardMacros.DoOnce` false :!label _label_4
          (:`Completed`
            (`self.DeathSequence`)))))))

(event `HandPreparationAndAttack`
  (bind _delta_seconds (`self.Delta Seconds`))
  (bind _as_player_hero_knight (`self.As Player Hero Knight`))
  (bind _delta_seconds_2 (`self.Delta Seconds`))
  (bind _as_player_hero_knight_2 (`self.As Player Hero Knight`))
  (bind (_returnvalue_x _returnvalue_y _returnvalue_z) (`KismetMathLibrary.BreakVector` (`self.K2_GetActorLocation` _as_player_hero_knight_2)))
  (bind (_returnvalue_x_2 _returnvalue_y_2 _returnvalue_z_2) (`KismetMathLibrary.BreakVector` (`SceneComponent.K2_GetComponentLocation` (`self.HandR`))))
  (bind (_returnvalue_x_3 _returnvalue_y_3 _returnvalue_z_3) (`KismetMathLibrary.BreakVector` (`SceneComponent.K2_GetComponentLocation` (`self.HandR`))))
  (bind (_returnvalue_x_4 _returnvalue_y_4 _returnvalue_z_4) (`KismetMathLibrary.BreakVector` (`self.K2_GetActorLocation` _as_player_hero_knight)))
  (bind (_returnvalue_x_5 _returnvalue_y_5 _returnvalue_z_5) (`KismetMathLibrary.BreakVector` (`SceneComponent.K2_GetComponentLocation` (`self.HandL`))))
  (bind (_returnvalue_x_6 _returnvalue_y_6 _returnvalue_z_6) (`KismetMathLibrary.BreakVector` (`SceneComponent.K2_GetComponentLocation` (`self.HandL`))))
  ;[1 0.05673 0.1564] Punch Hand for Attack Player
  (if (not (`self.IsRandomSideChoose`))
    ;;[1 0 0.7238] Choose Random Side
    (set `self.IsRandomSideChoose` true)
    (bind _output_get (set `self.IsRandomSide` (`KismetMathLibrary.Conv_IntToByte` (`KismetMathLibrary.RandomIntegerInRange` 0 1))))
    (switch `int` (`KismetMathLibrary.Conv_ByteToInt` _output_get)
      (:`0`
        (set `self.BossAttackHand` "NewEnumerator0"))
      (:`1`
        (set `self.BossAttackHand` "NewEnumerator2")))
    (else
      (set `self.BehaviourAI` "NewEnumerator1")
      (set `self.IsChooseAttack` true)))
  (switch `/Game/Assets/Blueprint/IA/Boss/BossAttackHand` (`self.BossAttackHand`)
    (:`NewEnumerator0`
      ;;[1 0.4581 0.1314] Attack L preparation
      (`/Engine/EditorBlueprintResources/StandardMacros.IsValid` _as_player_hero_knight
        (:`Is Valid`
          (`SceneComponent.K2_SetWorldLocation` (`self.HandL`) (`KismetMathLibrary.MakeVector` (`KismetMathLibrary.FInterpTo` _returnvalue_x_5 _returnvalue_x_4 _delta_seconds_2 1.0) (`KismetMathLibrary.FInterpTo` _returnvalue_y_5 (* _returnvalue_y_4 1.0) _delta_seconds_2 1.0) (`KismetMathLibrary.FInterpTo` _returnvalue_z_5 (* _returnvalue_z_4 0.3) _delta_seconds_2 1.0)) false false)
          (if (not (`self.IsPreprepared`))
            (set `self.IsPreprepared` true)
            (`KismetSystemLibrary.Delay` (`KismetMathLibrary.RandomFloatInRange` 5.0 10.0))
            (`PaperFlipbookComponent.SetFlipbook` (`self.Eyeflink`) "/Game/Assets/Sprite/Effects/Fire/Fire_Eyes.Fire_Eyes")
            (`KismetSystemLibrary.Delay` 0.5)
            (`PaperFlipbookComponent.SetFlipbook` (`self.Eyeflink`) null)
            (`GameplayStatics.PlaySound2D` "/Game/Assets/Audio/SFX/Boss/snd_b.snd_b" 1.0 1.0 0.0 null null)
            (`KismetSystemLibrary.Delay` 1.0)
            (set `self.BossAttackHand` "NewEnumerator1")
            (`self.EnabledCollision`)))))
    (:`NewEnumerator1`
      ;;[1 0.9886 0.1872] Attack  L
      (`/Engine/EditorBlueprintResources/StandardMacros.IsValid` (`self.As Player Hero Knight`)
        (:`Is Valid`
          (`SceneComponent.K2_SetWorldLocation` (`self.HandL`) (`KismetMathLibrary.MakeVector` _returnvalue_x_6 _returnvalue_y_6 (`KismetMathLibrary.FInterpTo` _returnvalue_z_6 -1027.193604 (`self.Delta Seconds`) 5.0)) false false)
          (if (not (`self.IsAttack`))
            (set `self.IsAttack` false)
            (`self.AttackSound`)
            (`KismetSystemLibrary.Delay` 3.0)
            (`self.ResetL`)
            (`self.AttackSoundEnabled`)))))
    (:`NewEnumerator2`
      ;;[0.313 1 0.04746] Attack L preparation
      (`/Engine/EditorBlueprintResources/StandardMacros.IsValid` _as_player_hero_knight_2
        (:`Is Valid`
          (`SceneComponent.K2_SetWorldLocation` (`self.HandR`) (`KismetMathLibrary.MakeVector` (`KismetMathLibrary.FInterpTo` _returnvalue_x_3 _returnvalue_x _delta_seconds 1.0) (`KismetMathLibrary.FInterpTo` _returnvalue_y_3 (* _returnvalue_y 1.0) _delta_seconds 1.0) (`KismetMathLibrary.FInterpTo` _returnvalue_z_3 (* _returnvalue_z 0.3) _delta_seconds 1.0)) false false)
          (if (not (`self.IsPreprepared`))
            (set `self.IsPreprepared` true)
            (`KismetSystemLibrary.Delay` (`KismetMathLibrary.RandomFloatInRange` 5.0 10.0))
            (`PaperFlipbookComponent.SetFlipbook` (`self.Eyeflink`) "/Game/Assets/Sprite/Effects/Fire/Fire_Eyes.Fire_Eyes")
            (`KismetSystemLibrary.Delay` 0.5)
            (`PaperFlipbookComponent.SetFlipbook` (`self.Eyeflink`) null)
            (`GameplayStatics.PlaySound2D` "/Game/Assets/Audio/SFX/Boss/snd_b.snd_b" 1.0 1.0 0.0 null null)
            (`KismetSystemLibrary.Delay` 1.0)
            (set `self.BossAttackHand` "NewEnumerator3")
            (`self.EnabledCollision`)))))
    (:`NewEnumerator3`
      ;;[0.04246 1 0.5093] Attack  L
      (`/Engine/EditorBlueprintResources/StandardMacros.IsValid` (`self.As Player Hero Knight`)
        (:`Is Valid`
          (`SceneComponent.K2_SetWorldLocation` (`self.HandR`) (`KismetMathLibrary.MakeVector` _returnvalue_x_2 _returnvalue_y_2 (`KismetMathLibrary.FInterpTo` _returnvalue_z_2 -1027.193604 (`self.Delta Seconds`) 5.0)) false false)
          (if (not (`self.IsAttack`))
            (set `self.IsAttack` false)
            (`self.AttackSound`)
            (`KismetSystemLibrary.Delay` 3.0)
            (`self.ResetR`)
            (`self.AttackSoundEnabled`)))))))

(event `ResetL`
  ;[1 0.2772 0.1573] Reset Hand Position & Logic Attack
  (`self.DisableCollision`)
  (set `self.IsPreprepared` false)
  (set `self.IsAttack` false)
  (set `self.BehaviourAI` "NewEnumerator0")
  (set `self.BossAttackHand` "NewEnumerator0")
  (`self.HandLTransformFreeze`)
  (set `self.IsRandomSideChoose` false)
  (set `self.IsRandomSide` 10)
  (`KismetSystemLibrary.Delay` 1.5 :!label _label_5)
  (set `self.IsChooseAttack` false))

(event `DebugResetDeath`
  (goto _label_4 :!via `Reset`))

(event `ResetR`
  ;[1 0.2772 0.1573] Reset Hand Position & Logic Attack
  (`self.DisableCollision`)
  (set `self.IsPreprepared` false)
  (set `self.IsAttack` false)
  (set `self.BehaviourAI` "NewEnumerator0")
  (set `self.BossAttackHand` "NewEnumerator2")
  (`self.HandRTransformFreeze`)
  (set `self.IsRandomSideChoose` false)
  (set `self.IsRandomSide` 10)
  (goto _label_5))

(event `Get Damaged Boss`
  (params (Damage :type "Float (double-precision)"))
  (bind _healthglobal (`self.HealthGlobal`))
  ;[1 0.3841 0.3642] Get Damage
  (if (not (`self.IsDeath`))
    (set `self.HealthGlobal` (- _healthglobal Damage))
    (`self.HitColor`)
    ;;[0.1198 0.004367 0.004367] Check if death
    (if (<= _healthglobal 0.0)
      (set `self.IsDeath` true)
      (bind _outactors (`GameplayStatics.GetAllActorsOfClass` "/Game/Assets/Blueprint/Environment/Niv3/BP_AudioCombat.BP_AudioCombat_C"))
      (for _array_element _outactors
        (`/Game/Assets/Blueprint/Environment/Niv3/BP_AudioCombat.FinishBoss` _array_element)
        (break)))))

(event `HitColor`
  ;[1 0.3385 0.3385] HitColor
  (`GameplayStatics.PlaySound2D` "/Game/Assets/Audio/SFX/Battle/15_Impact_flesh_02.15_Impact_flesh_02" 0.8 1.0 0.0 null null)
  (`PaperSpriteComponent.SetSpriteColor` (`self.Head`) (struct :`R` 0.537255 :`G` 0.078431 :`B` 0.078431 :`A` 1.0))
  (`PaperSpriteComponent.SetSpriteColor` (`self.HandR`) (struct :`R` 0.537255 :`G` 0.078431 :`B` 0.078431 :`A` 1.0))
  (`PaperSpriteComponent.SetSpriteColor` (`self.HandL`) (struct :`R` 0.537255 :`G` 0.078431 :`B` 0.078431 :`A` 1.0))
  (`KismetSystemLibrary.Delay` 0.1)
  (`PaperSpriteComponent.SetSpriteColor` (`self.Head`) (struct :`R` 1.0 :`G` 1.0 :`B` 1.0 :`A` 1.0))
  (`PaperSpriteComponent.SetSpriteColor` (`self.HandR`) (struct :`R` 1.0 :`G` 1.0 :`B` 1.0 :`A` 1.0))
  (`PaperSpriteComponent.SetSpriteColor` (`self.HandL`) (struct :`R` 1.0 :`G` 1.0 :`B` 1.0 :`A` 1.0)))

(event `self.HandR.OnComponentBeginOverlap`
  (params (OverlappedComponent :type "PrimitiveComponent Object Reference") (OtherActor :type "Actor Object Reference") (OtherComp :type "PrimitiveComponent Object Reference") (OtherBodyIndex :type Integer) (bFromSweep :type Boolean) (SweepResult :type "HitResult Structure (by ref)"))
  ;[0.003805 0.8903 1] CollisionsPlayer
  (bind _asplayer_hero_knight (cast `/Game/Assets/Blueprint/Player/PlayerHeroKnight` OtherActor)
    (:`then`
      (if (not (`/Game/Assets/Blueprint/Player/PlayerHeroKnight.IsAttack` _asplayer_hero_knight))
        (`/Game/Assets/Blueprint/Player/PlayerHeroKnight.GetDamaged` _asplayer_hero_knight (`KismetMathLibrary.RandomFloatInRange` 30.0 50.0))))
    (:`CastFailed`
      (bind _asbp_ennemie (cast `/Game/Assets/Blueprint/IA/BP_Ennemie` OtherActor))
      (`/Game/Assets/Blueprint/IA/BP_Ennemie.GetDamaged` _asbp_ennemie (`KismetMathLibrary.RandomFloatInRange` 60.0 120.0)))))

(event `DeathSequence`
  ;[0.716 1 0.2325] Death Sequence
  (if (`self.IsDeath`)
    (`self.SetMatToAllPart`)
    (`self.SpawnFlower`)
    (`KismetSystemLibrary.K2_SetTimer` null "DestroyBoss" 2.0)
    (`self.GetAllAIAndDestroy`)
    (else
      (`self.DebugResetDeath`))))

(event `AttackSound`
  (bind _returnvalue (`self.K2_GetActorLocation` (`self.As Player Hero Knight`)))
  (`/Engine/EditorBlueprintResources/StandardMacros.DoOnce` false :!label _label_6
    (:`Completed`
      (`GameplayStatics.PlaySound2D` "/Game/Assets/Audio/SFX/Boss/snd_grab.snd_grab" 1.0 1.0 0.0 null null)
      (`GameplayStatics.PlayWorldCameraShake` "/Game/Assets/Blueprint/FeedBack/CS_BossPunch.CS_BossPunch_C" _returnvalue 10000.0 10000.0)
      (`AddComponent|NODE_AddForceFeedbackComponent-0` :`RelativeTransform` (`KismetMathLibrary.MakeTransform` _returnvalue)))))

(event `AttackSoundEnabled`
  (goto _label_6 :!via `Reset`))

(event `EnabledCollision`
  ;[0.003805 0.8903 1] CollisionsPlayer
  (`PrimitiveComponent.SetCollisionResponseToAllChannels` (`self.HandR`) "ECR_Overlap")
  (`PrimitiveComponent.SetCollisionResponseToAllChannels` (`self.HandL`) "ECR_Overlap"))

(event `self.HandL.OnComponentBeginOverlap`
  (params (OverlappedComponent :type "PrimitiveComponent Object Reference") (OtherActor :type "Actor Object Reference") (OtherComp :type "PrimitiveComponent Object Reference") (OtherBodyIndex :type Integer) (bFromSweep :type Boolean) (SweepResult :type "HitResult Structure (by ref)"))
  ;[0.003805 0.8903 1] CollisionsPlayer
  (bind _asplayer_hero_knight (cast `/Game/Assets/Blueprint/Player/PlayerHeroKnight` OtherActor)
    (:`then`
      (if (not (`/Game/Assets/Blueprint/Player/PlayerHeroKnight.IsAttack` _asplayer_hero_knight))
        (`/Game/Assets/Blueprint/Player/PlayerHeroKnight.GetDamaged` _asplayer_hero_knight (`KismetMathLibrary.RandomFloatInRange` 30.0 50.0))))
    (:`CastFailed`
      (bind _asbp_ennemie (cast `/Game/Assets/Blueprint/IA/BP_Ennemie` OtherActor))
      (`/Game/Assets/Blueprint/IA/BP_Ennemie.GetDamaged` _asbp_ennemie (`KismetMathLibrary.RandomFloatInRange` 60.0 120.0)))))

(event `DisableCollision`
  ;[0.003805 0.8903 1] CollisionsPlayer
  (`PrimitiveComponent.SetCollisionResponseToAllChannels` (`self.HandR`) "ECR_Ignore")
  (`PrimitiveComponent.SetCollisionResponseToAllChannels` (`self.HandL`) "ECR_Ignore"))

(fn `DeathGoDown`
  (bind (_returnvalue_x _returnvalue_y _returnvalue_z) (`KismetMathLibrary.BreakVector` (`self.K2_GetActorLocation`)))
  (`self.K2_SetActorLocation` (`KismetMathLibrary.MakeVector` _returnvalue_x _returnvalue_y (`KismetMathLibrary.FInterpTo` _returnvalue_z -1500.0 (`self.Delta Seconds`) 2.0))))

(fn `DestroyBoss`
  (`PrimitiveComponent.SetMaterial` (`self.Head`) 0 "/Game/Assets/Material/M_Invisible.M_Invisible")
  (`PrimitiveComponent.SetMaterial` (`self.HandR`) 0 "/Game/Assets/Material/M_Invisible.M_Invisible")
  (`PrimitiveComponent.SetMaterial` (`self.HandL`) 0 "/Game/Assets/Material/M_Invisible.M_Invisible"))

(fn `FollowPlayer`
  (bind (_returnvalue_x _returnvalue_y _returnvalue_z) (`KismetMathLibrary.BreakVector` (`self.K2_GetActorLocation`)))
  (bind _as_player_hero_knight (`self.As Player Hero Knight`))
  (bind _delta_seconds (`self.Delta Seconds`))
  (bind (_returnvalue_x_2 _returnvalue_y_2 _returnvalue_z_2) (`KismetMathLibrary.BreakVector` (`self.K2_GetActorLocation` _as_player_hero_knight)))
  (`/Engine/EditorBlueprintResources/StandardMacros.IsValid` _as_player_hero_knight
    (:`Is Valid`
      (if (and (`|EnumInequality` (`self.BossAttackHand`) "NewEnumerator1") (`|EnumInequality` (`self.BossAttackHand`) "NewEnumerator3"))
        (`self.K2_SetActorLocation` (`KismetMathLibrary.MakeVector` (`KismetMathLibrary.FInterpTo` _returnvalue_x _returnvalue_x_2 _delta_seconds 1.0) _returnvalue_y (`KismetMathLibrary.FInterpTo` _returnvalue_z (* _returnvalue_z_2 0.8) _delta_seconds 1.0)))))))

(fn `GetAllAIAndDestroy`
  (bind _outactors (`GameplayStatics.GetAllActorsOfClass` "/Game/Assets/Blueprint/IA/BP_Ennemie.BP_Ennemie_C"))
  (if (!= (`KismetArrayLibrary.Array_Length` _outactors) 0)
    (for _array_element _outactors
      (`/Game/Assets/Blueprint/IA/BP_Ennemie.GetDamaged` _array_element 1000000.0))))

(fn `HandLTransformFreeze`
  (locals (NewLocalVar_0 :type "Vector Structure" :default (0.0 0.0 0.0)))
  (bind _delta_seconds (`self.Delta Seconds`))
  (bind (_returnvalue_x _returnvalue_y _returnvalue_z) (`KismetMathLibrary.BreakVector` (`SceneComponent.K2_GetComponentLocation` (`self.HandL`))))
  (bind (_returnvalue_x_2 _returnvalue_y_2 _returnvalue_z_2) (`KismetMathLibrary.BreakVector` (`SceneComponent.K2_GetComponentLocation` (`self.HandLPoint`))))
  (if (and (!= (`self.IsRandomSide`) 0) (not (`self.IsPreprepared`)))
    (`SceneComponent.K2_SetWorldLocation` (`self.HandL`) (`KismetMathLibrary.MakeVector` (`KismetMathLibrary.FInterpTo` _returnvalue_x _returnvalue_x_2 _delta_seconds 5.0) (`KismetMathLibrary.FInterpTo` _returnvalue_y _returnvalue_y_2 _delta_seconds 5.0) (`KismetMathLibrary.FInterpTo` _returnvalue_z _returnvalue_z_2 _delta_seconds 5.0)) false false)))

(fn `HandRTransformFreeze`
  (bind _delta_seconds (`self.Delta Seconds`))
  (bind (_returnvalue_x _returnvalue_y _returnvalue_z) (`KismetMathLibrary.BreakVector` (`SceneComponent.K2_GetComponentLocation` (`self.HandR`))))
  (bind (_returnvalue_x_2 _returnvalue_y_2 _returnvalue_z_2) (`KismetMathLibrary.BreakVector` (`SceneComponent.K2_GetComponentLocation` (`self.HandRPoint`))))
  (if (and (!= (`self.IsRandomSide`) 1) (not (`self.IsPreprepared`)))
    (`SceneComponent.K2_SetWorldLocation` (`self.HandR`) (`KismetMathLibrary.MakeVector` (`KismetMathLibrary.FInterpTo` _returnvalue_x _returnvalue_x_2 _delta_seconds 5.0) (`KismetMathLibrary.FInterpTo` _returnvalue_y _returnvalue_y_2 _delta_seconds 5.0) (`KismetMathLibrary.FInterpTo` _returnvalue_z _returnvalue_z_2 _delta_seconds 5.0)) false false)))

(fn `SetMatToAllPart`
  (`ActorComponent.K2_DestroyComponent` (`self.Eyeflink`))
  (`PrimitiveComponent.SetMaterial` (`self.Head`) 0 "/Game/Assets/Material/M_SpriteWave_Boss.M_SpriteWave_Boss")
  (`PrimitiveComponent.SetMaterial` (`self.HandR`) 0 "/Game/Assets/Material/M_SpriteWave_Boss.M_SpriteWave_Boss")
  (`PrimitiveComponent.SetMaterial` (`self.HandL`) 0 "/Game/Assets/Material/M_SpriteWave_Boss.M_SpriteWave_Boss"))

(fn `SpawnFlower`
  (`|SpawnActorFromClass` "/Game/Assets/Blueprint/GamePlay/Items/BP_Flower.BP_Flower_C" (`KismetMathLibrary.MakeTransform` (`self.K2_GetActorLocation`) (`self.K2_GetActorRotation`)) "AdjustIfPossibleButAlwaysSpawn" "OverrideRootScale" null null))

(fn `UserConstructionScript`)