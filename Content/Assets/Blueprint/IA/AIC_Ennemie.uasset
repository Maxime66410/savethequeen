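; AI controller for BP_Ennemie that runs the BT_Ennemie behavior tree and picks the player knight it targets.
; On possess it caches the pawn, then calls LoadOnAI, which is an empty event.
; When perception updates and the TargetActor blackboard key is unset, it scans sight-perceived PlayerHeroKnight actors for the nearest within a fixed range and writes it to that key.
; An existing valid target is never replaced here.
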(event `self.ReceiveBeginPlay`
  (`self.RunBehaviorTree` "/Game/Assets/Blueprint/IA/BT_Ennemie.BT_Ennemie")
  (set `self.BB` (`AIBlueprintHelperLibrary.GetBlackboard` null)))

(event `self.AIPerception.OnPerceptionUpdated`
  (params (UpdatedActors :type "Array of Actor Object Reference (by ref)"))
  (bind _returnvalue (`KismetMathLibrary.Vector_Distance` (`self.K2_GetActorLocation` (`self.BPENNEMIE`)) (`self.K2_GetActorLocation` (`self.Get BP`))))
  ;[1 1 1] Detect Enemie & Punch
  (`/Engine/EditorBlueprintResources/StandardMacros.IsValid` (`BlackboardComponent.GetValueAsObject` (`self.BB`) "TargetActor")
    (:`Is Not Valid`
      (set `self.Target Distance` 1000.0)
      (for _array_element (`AIPerceptionComponent.GetCurrentlyPerceivedActors` (`self.AIPerception`) "/Script/AIModule.AISense_Sight")
        (bind _asplayer_hero_knight (cast `/Game/Assets/Blueprint/Player/PlayerHeroKnight` _array_element))
        (set `self.Get BP` _asplayer_hero_knight)
        (if (> (`self.Target Distance`) _returnvalue)
          (set `self.Target Distance` _returnvalue)
          (`BlackboardComponent.SetValueAsObject` (`self.BB`) "TargetActor" (`self.Get BP`)))))))

(event `self.ReceivePossess`
  (params (PossessedPawn :type "Pawn Object Reference"))
  ;[1 1 1] Detect Enemie & Punch
  (bind _asbp_ennemie (cast `/Game/Assets/Blueprint/IA/BP_Ennemie` PossessedPawn))
  (set `self.BPENNEMIE` _asbp_ennemie)
  (`self.Load on AI`))

(event `Load on AI`)

(fn `UserConstructionScript`)