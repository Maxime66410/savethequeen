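; Paper2D side-scroller enemy that chases and melees PlayerHeroKnight, takes damage, and dies with a timed disappear.
; A self-rescheduling AI MoveTo loop follows the target set by the TargetPlayer overlap or by being hit, attacking on arrival through a briefly enabled overlap box.
; Tick picks flipbooks, snaps facing left or right and locks Y.
; JumpSmart offers arc-based launches; a random TypeGuard at spawn selects the attack flipbook.
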(event `MoveToPlayer`
  (bind _as_player_hero_knight (`self.As Player Hero Knight`))
  ;[1 1 1] Move to Player & Attack
  (if (not (`self.Is Death`))
    (if (not (`self.IsGetDamage`))
      (`/Engine/EditorBlueprintResources/StandardMacros.IsValid` _as_player_hero_knight
        (:`Is Valid`
          (if (not (`self.Is Death`))
            (bind _asaicontroller (cast `AIController` (`self.GetController`)))
            (bind _returnvalue (`AIController.MoveToActor` _asaicontroller _as_player_hero_knight 1.0 true true true null true))
            (set `self.StatuesPlayerMove` _returnvalue)
            (if (`|EnumEquality` (`self.StatuesPlayerMove`) "AlreadyAtGoal")
              (if (not (`self.Is Attack`))
                (`self.AttackPlayer`))
              (`KismetSystemLibrary.Delay` 0.2 :!label _label)
              (`self.MoveToPlayer`)
              (elif (not (`self.Is Death`))
                (goto _label)))))
        (:`Is Not Valid`
          (goto _label)))
      (else
        (goto _label)))))

(event `UpdateAnimation`
  ;[1 1 1] Update animation
  (if (not (`self.Is Attack`))
    (if (not (`self.IsGetDamage`))
      (if (not (`self.Is Death`))
        (`PaperFlipbookComponent.SetFlipbook` (`self.Sprite`) (select `bool` (`NavMovementComponent.IsFalling` (`self.CharacterMovement`)) :`false` (select `bool` (> (`KismetMathLibrary.VSize` (`self.GetVelocity`)) 0.0) :`false` "/Game/Assets/Sprite/Ennemy/Idle/Ennemie_Idle.Ennemie_Idle" :`true` "/Game/Assets/Sprite/Ennemy/Run/Ennemie_Run.Ennemie_Run" :!type "PaperFlipbook Object Reference") :`true` "/Game/Assets/Sprite/Ennemy/Fall/Ennemie_Fall.Ennemie_Fall"))
        (else
          (bind _asaicontroller (cast `AIController` (`self.GetController`)))
          (`AIController.MoveToActor` _asaicontroller _asaicontroller 1.0 true true true null true))))))

(event `AttackPlayer`
  ;[1 0.6558 0.4623] Attack
  (if (not (`self.Is Death`))
    (if (not (`/Game/Assets/Blueprint/Player/PlayerHeroKnight.IsDeath` (`self.As Player Hero Knight`)))
      (if (not (`self.Is Attack`))
        (set `self.Is Attack` true)
        (`PaperFlipbookComponent.SetFlipbook` (`self.Sprite`) (`|GetArrayItem` (`self.AttackStates`) (`KismetMathLibrary.Conv_ByteToInt` (`self.TypeGuard`))))
        (`KismetSystemLibrary.Delay` 0.3)
        (if (not (`self.IsGetDamage`))
          (`PrimitiveComponent.SetCollisionResponseToAllChannels` (`self.Trigger Attack Box`) "ECR_Overlap")
          (`KismetSystemLibrary.Delay` 0.2))
        (`PrimitiveComponent.SetCollisionResponseToAllChannels` (`self.Trigger Attack Box`) "ECR_Ignore")
        (`PaperFlipbookComponent.SetFlipbook` (`self.Sprite`) "/Game/Assets/Sprite/Ennemy/Idle/Ennemie_Idle.Ennemie_Idle")
        (`KismetSystemLibrary.Delay` 0.2)
        (set `self.Is Attack` false)))))

(event `self.ReceiveBeginPlay`
  ;[1 1 1] Start Player
  (`ActorComponent.SetIsReplicated` (`self.Sprite`) true)
  (set `self.TypeGuard` (`KismetMathLibrary.Conv_IntToByte` (`KismetMathLibrary.RandomIntegerInRange` 0 3)))
  (`self.MoveToPlayer`)
  (`PrimitiveComponent.SetCollisionResponseToAllChannels` (`self.Trigger Attack Box`) "ECR_Ignore"))

(event `self.Trigger Attack Box.OnComponentBeginOverlap`
  (params (OverlappedComponent :type "PrimitiveComponent Object Reference") (OtherActor :type "Actor Object Reference") (OtherComp :type "PrimitiveComponent Object Reference") (OtherBodyIndex :type Integer) (bFromSweep :type Boolean) (SweepResult :type "HitResult Structure (by ref)"))
  ;[1 1 1] Attack Player if in box
  (bind _asplayer_hero_knight (cast `/Game/Assets/Blueprint/Player/PlayerHeroKnight` OtherActor))
  (if (not (`self.Is Death`))
    (if (`self.Is Attack`)
      (`/Game/Assets/Blueprint/Player/PlayerHeroKnight.GetDamaged` _asplayer_hero_knight (`KismetMathLibrary.RandomFloatInRange` 2.0 10.0)))))

(event `AlwaysOnZ`
  (bind (_returnvalue_x _returnvalue_y _returnvalue_z) (`KismetMathLibrary.BreakVector` (`self.K2_GetActorLocation`)))
  ;[1 1 1] Fix Z Position
  (`self.K2_SetActorLocation` (`KismetMathLibrary.MakeVector` _returnvalue_x (`self.FreezeLocationY`) _returnvalue_z)))

(event `self.ReceiveTick`
  (params (DeltaSeconds :type "Float (single-precision)"))
  ;[1 1 1] Rotator Flip
  (set `self.Delta Seconds` DeltaSeconds)
  (`self.UpdateAnimation`)
  (`/Engine/EditorBlueprintResources/StandardMacros.CompareFloat` (.x (`self.GetActorForwardVector`))
    (:`>`
      (`self.K2_SetActorRotation` (`KismetMathLibrary.MakeRotator` 0.0)))
    (:`<`
      (`self.K2_SetActorRotation` (`KismetMathLibrary.MakeRotator` 0.0 0.0 180.0))))
  (`self.AlwaysOnZ`))

(event `GetDamaged`
  (params (Damage :type "Float (double-precision)"))
  (bind _capsulecomponent (`self.CapsuleComponent`))
  ;[1 0.2603 0] Get Damage
  (if (not (`self.Is Death`))
    (`GameplayStatics.PlaySound2D` "/Game/Assets/Audio/SFX/Battle/15_Impact_flesh_02.15_Impact_flesh_02" 0.5 (`KismetMathLibrary.RandomFloatInRange` 0.8 1.2) 0.0 null null)
    (set `self.IsGetDamage` true)
    (`PaperFlipbookComponent.SetFlipbook` (`self.Sprite`) "/Game/Assets/Sprite/Ennemy/Hit/Ennemie_Hit.Ennemie_Hit")
    (set `self.Health` (- (`self.Health`) Damage))
    (`KismetSystemLibrary.Delay` 0.1)
    (if (>= 0.0 (`self.Health`))
      (set `self.Is Death` true)
      (`PaperFlipbookComponent.SetFlipbook` (`self.Sprite`) "/Game/Assets/Sprite/Ennemy/Death/Ennemie_Death.Ennemie_Death")
      (`KismetSystemLibrary.Delay` 0.5)
      (`GameplayStatics.PlaySound2D` "/Game/Assets/Audio/SFX/Battle/69_Enemy_death_01.69_Enemy_death_01" 1.0 1.0 0.0 null null)
      (`PaperFlipbookComponent.SetFlipbook` (`self.Sprite`) "/Game/Assets/Sprite/Ennemy/Death/Ennemie_Death_Loop.Ennemie_Death_Loop")
      (`CapsuleComponent.SetCapsuleRadius` _capsulecomponent 13.251322 true)
      (`CapsuleComponent.SetCapsuleHalfHeight` _capsulecomponent 13.251322 true)
      (`PrimitiveComponent.SetCollisionResponseToChannel` (`self.CapsuleComponent`) "ECC_Pawn" "ECR_Ignore")
      (`KismetSystemLibrary.Delay` 5.0)
      (`PaperFlipbookComponent.SetFlipbook` (`self.Sprite`) "/Game/Assets/Sprite/Ennemy/Disappear/Ennemie_Disappear.Ennemie_Disappear")
      (`KismetSystemLibrary.Delay` 1.0)
      (`self.K2_DestroyActor`)
      (else
        (`KismetSystemLibrary.Delay` 0.2)
        (bind _asplayer_hero_knight (cast `/Game/Assets/Blueprint/Player/PlayerHeroKnight` (`GameplayStatics.GetPlayerCharacter` 0)))
        (set `self.As Player Hero Knight` _asplayer_hero_knight)
        (set `self.IsGetDamage` false)))))

(event `self.TargetPlayer.OnComponentBeginOverlap`
  (params (OverlappedComponent :type "PrimitiveComponent Object Reference") (OtherActor :type "Actor Object Reference") (OtherComp :type "PrimitiveComponent Object Reference") (OtherBodyIndex :type Integer) (bFromSweep :type Boolean) (SweepResult :type "HitResult Structure (by ref)"))
  ;[1 1 1] Trigger / Exit Player
  (bind _asplayer_hero_knight (cast `/Game/Assets/Blueprint/Player/PlayerHeroKnight` OtherActor))
  (if (not (`self.Is Death`))
    (set `self.As Player Hero Knight` _asplayer_hero_knight)))

(event `JumpSmart`
  (params (Destination :type "Vector Structure") (JumpPower :type "Float (double-precision)"))
  ;[1 1 1] Smart Jump
  (if (not (`self.Is Attack`))
    (if (not (`self.Isjump`))
      (set `self.Isjump` true)
      (bind _outlaunchvelocity (`GameplayStatics.SuggestProjectileVelocity_CustomArc` (`self.K2_GetActorLocation`) Destination))
      (bind (_returnvalue_x _returnvalue_y _returnvalue_z) (`KismetMathLibrary.BreakVector` (* _outlaunchvelocity JumpPower)))
      (`self.LaunchCharacter` (`KismetMathLibrary.MakeVector` _returnvalue_x -355.0 _returnvalue_z) true true)
      (`GameplayStatics.PlaySound2D` "/Game/Assets/Audio/SFX/Movement/30_Jump_03.30_Jump_03" 0.5 1.0 0.0 null null)
      (`KismetSystemLibrary.Delay` 2.0)
      (set `self.Isjump` false))))

(event `self.TargetPlayer.OnComponentEndOverlap`
  (params (OverlappedComponent :type "PrimitiveComponent Object Reference") (OtherActor :type "Actor Object Reference") (OtherComp :type "PrimitiveComponent Object Reference") (OtherBodyIndex :type Integer))
  ;[1 1 1] Trigger / Exit Player
  (cast `/Game/Assets/Blueprint/Player/PlayerHeroKnight` OtherActor)
  (if (not (`self.Is Death`))
    (set `self.As Player Hero Knight` null)))

(fn `UserConstructionScript`)